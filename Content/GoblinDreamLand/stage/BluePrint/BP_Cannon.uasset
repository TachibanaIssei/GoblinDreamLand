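; BP_Cannon is a stage cannon that repeatedly fires bursts of three BP_StoneBall projectiles.
; A looping timer starts each burst through a second timer that calls Resize, which counts shots and clears itself after the third.
; Each shot plays a timeline that animates the actor's X scale and spawns the ball at the Muzzle socket on an event track.
; Overlaps set TouchFloor, but the manual gravity logic using it is unconnected.
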(event `self.ReceiveBeginPlay`
  (`KismetSystemLibrary.K2_SetTimerDelegate` (delegate `ResizeEvent`) 3.5 true) ; 3秒ごとにResizeEventイベントを行う
)

(event `ResizeEvent`
  (bind _returnvalue (`KismetSystemLibrary.K2_SetTimer` null "Resize" 0.5 true)) ; 0.5秒ごとにResize関数を呼び出す
  (set `self.TimerHandle` _returnvalue))

(event `ResizeCannon`
  (bind (_direction _cannonscale) (`Timeline|タイムライン` :!via `PlayFromStart`)
    (:`Update`
      ;[1 1 1] 大砲の大きさを変更
      (`self.SetActorScale3D` (`KismetMathLibrary.MakeVector` _cannonscale 1.0 1.0)))
    (:`FireBall`
      (`self.FireProjectile`) ; 弾の発射
    )))

(event `self.ReceiveTick`
  (params (DeltaSeconds :type "Float (single-precision)")))

(event `self.ReceiveActorBeginOverlap`
  (params (OtherActor :type "Actor Object Reference"))
  ;[1 1 1] 床についているかどうかを設定
  (set `self.TouchFloor` true))

(event `self.ReceiveActorEndOverlap`
  (params (OtherActor :type "Actor Object Reference"))
  ;[1 1 1] 床についているかどうかを設定
  (set `self.TouchFloor` false))

(fn `FireProjectile`
  ;[1 1 1] 弾の生成
  (`|SpawnActorFromClass` "/Game/GoblinDreamLand/stage/BluePrint/BP_StoneBall.BP_StoneBall_C" (`SceneComponent.GetSocketTransform` (`self.Cannon`) "Muzzle" "RTS_World") "Undefined" "MultiplyWithRoot" null null))

(fn `Resize`
  (`self.ResizeCannon`)
  ;[1 1 1] 発生させた弾の数を記憶
  (set `self.ShotsFired` (+ (`self.ShotsFired`) 1))
  ;[1 1 1] 3つ発生させたらカウントをリセット
  (if (>= (`self.ShotsFired`) 3)
    (`KismetSystemLibrary.K2_ClearTimer` null "Resize")
    (set `self.ShotsFired` 0)))

(fn `UserConstructionScript`)