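; Goblin wizard enemy character that attacks by casting fireballs and leaves a wand behind when it drops its weapon.
; Attack plays a montage whose notify spawns a BP_FireBall ahead of the goblin and sets its projectile velocity from the forward vector and FireSpeed.
; Montage completion or interruption signals attack end.
; The DropWeapon override runs the parent logic, spawns BP_Spwan_Wand at the goblin's transform and stops the attack montage.
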(event `self.Attack`
  (`|PlayMontage` (`self.Mesh`) "/Game/GoblinDreamLand/Core/Characters/Goblin_AI/Goblin_Wizard/Animation/Anim_Goblin_Wizard_attack_01_Montage.Anim_Goblin_Wizard_attack_01_Montage"
    (:`OnCompleted`
      (`self.OnAttackEnd` :!label _label))
    (:`OnInterrupted`
      (goto _label))
    (:`OnNotifyBegin`
      (bind _returnvalue (`|SpawnActorFromClass` "/Game/GoblinDreamLand/Core/Characters/Goblin_AI/Niagara/BP_FireBall.BP_FireBall_C" (`KismetMathLibrary.Conv_VectorToTransform` (+ (`self.K2_GetActorLocation`) (* (`self.GetActorForwardVector`) (`self.Distance`)))) "Undefined" "MultiplyWithRoot" null null))
      (`ProjectileMovementComponent.SetVelocityInLocalSpace` (`/Game/GoblinDreamLand/Core/Characters/Goblin_AI/Niagara/BP_FireBall.ProjectileMovement` _returnvalue) (* (`self.GetActorForwardVector`) (`self.FireSpeed`))))))

(fn `DropWeapon`
  (`parent.DropWeapon`)
  (`|SpawnActorFromClass` "/Game/GoblinDreamLand/Core/Characters/Goblin_AI/Weapon/Spawn/BP_Spwan_Wand.BP_Spwan_Wand_C" (`self.GetTransform`) "Undefined" "MultiplyWithRoot" null null)
  (`self.StopAnimMontage` "/Game/GoblinDreamLand/Core/Characters/Goblin_AI/Goblin_Wizard/Animation/Anim_Goblin_Wizard_attack_01_Montage.Anim_Goblin_Wizard_attack_01_Montage"))

(fn `UserConstructionScript`
  (`parent.UserConstructionScript`))