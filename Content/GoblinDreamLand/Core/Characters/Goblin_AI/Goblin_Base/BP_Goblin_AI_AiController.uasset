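; AI controller for the goblin enemy that starts its behavior tree and feeds player perception into the blackboard.
; On BeginPlay it sets up the base goblin blackboard, clears TargetLocation and runs the base goblin behavior tree.
; Perception updates for the first player character store it in TargetPlayer when sensed.
; Losing the player clears a differently named key, Player, leaving TargetPlayer set.
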(event `self.ReceiveBeginPlay`
  (bind _blackboardcomponent (`self.UseBlackboard` "/Game/GoblinDreamLand/Core/Characters/Goblin_AI/Goblin_Base/BB_Goblin_AI_base.BB_Goblin_AI_base"))
  (`BlackboardComponent.SetValueAsObject` _blackboardcomponent "TargetLocation" null)
  (`self.RunBehaviorTree` "/Game/GoblinDreamLand/Core/Characters/Goblin_AI/Goblin_Base/BT_Goblin_AI_base.BT_Goblin_AI_base"))

(event `self.AIPerception.OnTargetPerceptionUpdated`
  (params (Actor :type "Actor Object Reference") (Stimulus :type "AIStimulus Structure"))
  (if (== Actor (`GameplayStatics.GetPlayerCharacter` 0))
    (if (`.bSuccessfullySensed` (break `AIStimulus` Stimulus))
      (`BlackboardComponent.SetValueAsObject` (`self.Blackboard`) "TargetPlayer" Actor)
      (else
        (`BlackboardComponent.SetValueAsObject` (`self.Blackboard`) "Player" null)))))

(fn `UserConstructionScript`)