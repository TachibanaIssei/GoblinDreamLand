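; BP_Apple is an apple actor that bobs around its spawn point and destroys itself when any actor begins overlapping it.
; BeginPlay stores the initial location, and Tick adds a sine offset driven by accumulated time, Frequency and Amplitude.
; The sine phase also includes the scaled sum of the current location's coordinates, so apples at different positions float out of sync.
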(event `self.ReceiveBeginPlay`
  ;[1 1 1] 初期座標の設定
  (set `self.FirstPosition` (`self.K2_GetActorLocation`)))

(event `self.ReceiveTick`
  (params (DeltaSeconds :type "Float (single-precision)"))
  ;[1 1 1] 経過時間の測定
  (bind _output_get (set `self.Time` (+ DeltaSeconds (`self.Time`))))
  ;[1 1 1] 初期座標に求めた振れ幅を加算して最終的な座標を求める
  (`self.K2_SetActorLocation` (+ (`self.FirstPosition`) (* (`KismetMathLibrary.Sin` (+ (* _output_get (`self.Frequency`)) (* (+ (+ (.x (`self.K2_GetActorLocation`)) (.y (`self.K2_GetActorLocation`))) (.z (`self.K2_GetActorLocation`))) 0.03))) (`self.Amplitude`)))))

(event `self.ReceiveActorBeginOverlap`
  (params (OtherActor :type "Actor Object Reference"))
  (`self.K2_DestroyActor`))

(fn `UserConstructionScript`)