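; BP_PlayerNormal is a player character with punch and tackle attacks, triggered from Enhanced Input by activating Gameplay Ability System abilities by tag.
; Left and right weapon collision overlaps apply fixed damage and spawn a Niagara hit effect at the hit actor's root, pitched toward the player mesh.
; The tackle collision instead calls HitTackle on BP_TestEnemy.
; Each collider uses its own DoOnce with a delayed reset to throttle repeat hits.
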(event `self.WeaponRCollision.OnComponentBeginOverlap`
  (params (OverlappedComponent :type "PrimitiveComponent Object Reference") (OtherActor :type "Actor Object Reference") (OtherComp :type "PrimitiveComponent Object Reference") (OtherBodyIndex :type Integer) (bFromSweep :type Boolean) (SweepResult :type "HitResult Structure (by ref)"))
  ;[1 1 1] 武器コリジョンに当たるとダメージを与える
  (`/Engine/EditorBlueprintResources/StandardMacros.DoOnce` false :!label _label
    (:`Completed`
      (`GameplayStatics.ApplyDamage` OtherActor 10.0)
      (`self.NewFunction_0` (`Actor.RootComponent` OtherActor))
      (`KismetSystemLibrary.Delay` 0.5)
      (goto _label :!via `Reset`))))

(event `self.WeaponLCollision.OnComponentBeginOverlap`
  (params (OverlappedComponent :type "PrimitiveComponent Object Reference") (OtherActor :type "Actor Object Reference") (OtherComp :type "PrimitiveComponent Object Reference") (OtherBodyIndex :type Integer) (bFromSweep :type Boolean) (SweepResult :type "HitResult Structure (by ref)"))
  ;[1 1 1] 武器コリジョンに当たるとダメージを与える
  (`/Engine/EditorBlueprintResources/StandardMacros.DoOnce` false :!label _label_2
    (:`Completed`
      (`GameplayStatics.ApplyDamage` OtherActor 10.0)
      (`self.NewFunction_0` (`Actor.RootComponent` OtherActor))
      (`KismetSystemLibrary.Delay` 0.5)
      (goto _label_2 :!via `Reset`))))

(event `self.TackleCollision.OnComponentBeginOverlap`
  (params (OverlappedComponent :type "PrimitiveComponent Object Reference") (OtherActor :type "Actor Object Reference") (OtherComp :type "PrimitiveComponent Object Reference") (OtherBodyIndex :type Integer) (bFromSweep :type Boolean) (SweepResult :type "HitResult Structure (by ref)"))
  ;[1 1 1] タックルの当たり判定
  (`/Engine/EditorBlueprintResources/StandardMacros.DoOnce` false :!label _label_3
    (:`Completed`
      (bind _asbp_test_enemy (cast `/Game/GoblinDreamLand/Core/Characters/Player/BP/BP_TestEnemy` OtherActor))
      (`/Game/GoblinDreamLand/Core/Characters/Player/BP/BP_TestEnemy.HitTackle` _asbp_test_enemy)
      (`KismetSystemLibrary.Delay` 0.5)
      (goto _label_3 :!via `Reset`))))

(event `EnhancedInput|/Game/GoblinDreamLand/Core/Interactables/IA_Punch`
  (params (ActionValue :type Boolean) (ElapsedSeconds :type "Float (double-precision)") (TriggeredSeconds :type "Float (double-precision)") (InputAction :type "InputAction Object Reference" :default "/Game/GoblinDreamLand/Core/Interactables/IA_Punch.IA_Punch"))
  ;[1 1 1] 3連パンチ
  (:`Started`
    (`AbilitySystemComponent.TryActivateAbilitiesByTag` (`self.AbilitySystem`) (`BlueprintGameplayTagLibrary.MakeLiteralGameplayTagContainer` (struct :`GameplayTags` (struct :`(TagName` "Ability.Attack.Punch")))) true)))

(event `EnhancedInput|/Game/GoblinDreamLand/Core/Interactables/IA_CopyAttack`
  (params (ActionValue :type Boolean) (ElapsedSeconds :type "Float (double-precision)") (TriggeredSeconds :type "Float (double-precision)") (InputAction :type "InputAction Object Reference" :default "/Game/GoblinDreamLand/Core/Interactables/IA_CopyAttack.IA_CopyAttack"))
  ;[1 1 1] タックル
  (:`Started`
    (`AbilitySystemComponent.TryActivateAbilitiesByTag` (`self.AbilitySystem`) (`BlueprintGameplayTagLibrary.MakeLiteralGameplayTagContainer` (struct :`GameplayTags` (struct :`(TagName` "Ability.Attack.Tackle")))) true)))

(fn `NewFunction_0`
  (params (CollisionComponent :type "SceneComponent Object Reference"))
  (bind _returnvalue (`SceneComponent.K2_GetComponentLocation` CollisionComponent))
  (`NiagaraFunctionLibrary.SpawnSystemAtLocation` "/Game/GoblinDreamLand/Effects/NS_Punchi_Hit1.NS_Punchi_Hit1" _returnvalue (`KismetMathLibrary.MakeRotator` 90.0 (.pitch (`KismetMathLibrary.FindLookAtRotation` _returnvalue (`SceneComponent.K2_GetComponentLocation` (`self.Mesh`)))) 90.0)))

(fn `UserConstructionScript`
  (`parent.UserConstructionScript`))