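; Player controller that lets the player switch between a normal goblin and a sword goblin character.
; On BeginPlay it adds the input mapping and spawns the sword goblin hidden, attached to the normal pawn.
; NormaltoSword and SwordtoNormal swap them after a short delay: detach, match transform, toggle visibility, collision and movement, reattach the hidden one, then possess the active one.
; It tracks the active form, exposed through GetNowType.
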(event `self.ReceiveBeginPlay`
  (bind _returnvalue (pcsubsystem `EnhancedInputLocalPlayerSubsystem` (`GameplayStatics.GetPlayerController` 0)))
  (`/Engine/EditorBlueprintResources/StandardMacros.IsValid` _returnvalue
    (:`Is Valid`
      (`EnhancedInputSubsystemInterface.AddMappingContext` _returnvalue "/Game/GoblinDreamLand/Core/Interactables/IMC_Default.IMC_Default" 0 (struct))
      (bind _asbp_player_normal (cast `/Game/GoblinDreamLand/Core/Characters/Player/BP/BP_PlayerNormal` (`GameplayStatics.GetPlayerPawn` 0)))
      (set `self.NormalGoblinPlayer` _asbp_player_normal)
      (set `self.PlayerType` "NewEnumerator0")
      (bind _returnvalue_2 (`|SpawnActorFromClass` "/Game/GoblinDreamLand/Core/Characters/Player/BP/BP_PlayerSword.BP_PlayerSword_C" (`KismetMathLibrary.MakeTransform` (0.0 0.0 0.0)) "Undefined" "MultiplyWithRoot" null null))
      (set `self.SwordGoblinPlayer` _returnvalue_2)
      (`self.Set Character Visibility and Collision` false (`self.SwordGoblinPlayer`))
      (`self.K2_SetActorTransform` (`self.SwordGoblinPlayer`) (`self.GetTransform` (`self.NormalGoblinPlayer`)) false false)
      (`self.K2_AttachToActor` (`self.SwordGoblinPlayer`) (`self.NormalGoblinPlayer`) "None" "KeepRelative" "KeepRelative" "KeepRelative" true))))

(event `/Game/GoblinDreamLand/Core/Characters/Player/BP/IF_ChangePlayerType.NormalToSword`
  (`KismetSystemLibrary.Delay` 0.2)
  (`self.K2_DetachFromActor` (`self.SwordGoblinPlayer`) "KeepRelative" "KeepRelative" "KeepRelative") ; アタッチを切り離す
  (`self.K2_SetActorTransform` (`self.SwordGoblinPlayer`) (`self.GetTransform` (`self.NormalGoblinPlayer`)) false false)
  (`self.Set Character Visibility and Collision` false (`self.NormalGoblinPlayer`))
  (`self.Set Character Visibility and Collision` true (`self.SwordGoblinPlayer`))
  (`self.K2_AttachToActor` (`self.NormalGoblinPlayer`) (`self.SwordGoblinPlayer`) "None" "KeepRelative" "KeepRelative" "KeepRelative" true) ; ノーマルを剣士についてくるようにアタッチ
  (`self.Possess` (`self.SwordGoblinPlayer`)) ; 操作プレイヤー変更
  (set `self.PlayerType` "NewEnumerator1"))

(event `/Game/GoblinDreamLand/Core/Characters/Player/BP/IF_ChangePlayerType.SwordToNormal`
  (`KismetSystemLibrary.Delay` 0.2)
  (`self.K2_DetachFromActor` (`self.NormalGoblinPlayer`) "KeepRelative" "KeepRelative" "KeepRelative") ; アタッチを切り離す
  (`self.K2_SetActorTransform` (`self.NormalGoblinPlayer`) (`self.GetTransform` (`self.SwordGoblinPlayer`)) false false)
  (`self.Set Character Visibility and Collision` false (`self.SwordGoblinPlayer`))
  (`self.Set Character Visibility and Collision` true (`self.NormalGoblinPlayer`))
  (`self.K2_AttachToActor` (`self.SwordGoblinPlayer`) (`self.NormalGoblinPlayer`) "None" "KeepRelative" "KeepRelative" "KeepRelative" true) ; ついてくるようにアタッチ
  (`self.Possess` (`self.NormalGoblinPlayer`)) ; 操作プレイヤー変更
  (set `self.PlayerType` "NewEnumerator0"))

(fn `GetNowType`
  (returns (PlayerType :type "/Game/GoblinDreamLand/Core/Characters/Player/EN_PlayerType Enum"))
  (return (`self.PlayerType`)))

(fn `Set Character Visibility and Collision`
  (params (VisibilityAndCollision :type Boolean) (Character :type "Character Object Reference"))
  (locals (TargetCharacter :type "Character Object Reference"))
  (set `local.TargetCharacter` Character)
  (if VisibilityAndCollision
    ;[1 1 1] 見える、当たり判定がある
    (`SceneComponent.SetVisibility` (`Character.Mesh` (`local.TargetCharacter`)) true true)
    (`PrimitiveComponent.SetCollisionEnabled` (`Character.CapsuleComponent` (`local.TargetCharacter`)) "QueryAndPhysics")
    (`PrimitiveComponent.SetCollisionEnabled` (`Character.Mesh` (`local.TargetCharacter`)) "QueryAndPhysics")
    (`CharacterMovementComponent.SetMovementMode` (`Character.CharacterMovement` (`local.TargetCharacter`)) "MOVE_Walking" 0)
    (else
      ;[1 1 1] 見えない、当たり判定がない
      (`SceneComponent.SetVisibility` (`Character.Mesh` (`local.TargetCharacter`)) false true)
      (`PrimitiveComponent.SetCollisionEnabled` (`Character.CapsuleComponent` (`local.TargetCharacter`)) "NoCollision")
      (`PrimitiveComponent.SetCollisionEnabled` (`Character.Mesh` (`local.TargetCharacter`)) "NoCollision")
      (`CharacterMovementComponent.DisableMovement` (`Character.CharacterMovement` (`local.TargetCharacter`))))))

(fn `UserConstructionScript`)