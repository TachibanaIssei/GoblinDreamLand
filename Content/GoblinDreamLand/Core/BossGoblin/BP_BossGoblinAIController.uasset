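; AI controller for the boss goblin, which runs its behavior tree and mirrors combat state into the blackboard.
; BeginPlay stores the player and starts the tree; events set the field-entry and attacking flags or stop the logic.
; For tackles it locks the direction to the player at the start, switches the pawn's speed and acceleration, drives straight or backward movement, then restores defaults.
; Tick publishes the forward vector while IsBattleStart is true.
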(event `StopControl`
  (`BrainComponent.StopLogic` (`self.BrainComponent`) "") ; ビヘイビアツリーの動きを止める
)

(event `攻撃中にする`
  ;[1 1 1] 攻撃フラグの処理
  (bind _blackboardcomponent (`self.UseBlackboard` "/Game/GoblinDreamLand/Core/BossGoblin/BB_BossGoblin.BB_BossGoblin"))
  (`BlackboardComponent.SetValueAsBool` _blackboardcomponent "IsAttacking" true))

(event `攻撃を終わる`
  ;[1 1 1] 攻撃フラグの処理
  (bind _blackboardcomponent (`self.UseBlackboard` "/Game/GoblinDreamLand/Core/BossGoblin/BB_BossGoblin.BB_BossGoblin"))
  (`BlackboardComponent.SetValueAsBool` _blackboardcomponent "IsAttacking" false))

(event `self.ReceiveBeginPlay`
  (bind _returnvalue (`GameplayStatics.GetPlayerCharacter` 0))
  ;[1 1 1] 初期化処理
  (bind _blackboardcomponent (`self.UseBlackboard` "/Game/GoblinDreamLand/Core/BossGoblin/BB_BossGoblin.BB_BossGoblin"))
  (`/Engine/EditorBlueprintResources/StandardMacros.IsValid` _returnvalue
    (:`Is Valid`
      (`BlackboardComponent.SetValueAsObject` _blackboardcomponent "Player" _returnvalue)
      (`self.RunBehaviorTree` "/Game/GoblinDreamLand/Core/BossGoblin/BT_BossGoblin.BT_BossGoblin"))))

(event `RunStartBehaviorTree`
  ;[0.04 1 0.01286] ビヘイビアツリーの管理開始
  (bind _blackboardcomponent (`self.UseBlackboard` "/Game/GoblinDreamLand/Core/BossGoblin/BB_BossGoblin.BB_BossGoblin"))
  (`BlackboardComponent.SetValueAsBool` _blackboardcomponent "IsEntryPlayerToField" true))

(event `self.ReceiveTick`
  (params (DeltaSeconds :type "Float (single-precision)"))
  ;[1 1 1] 毎フレーム更新処理
  (if (`self.IsBattleStart`)
    (bind _blackboardcomponent (`self.UseBlackboard` "/Game/GoblinDreamLand/Core/BossGoblin/BB_BossGoblin.BB_BossGoblin"))
    (`BlackboardComponent.SetValueAsVector` _blackboardcomponent "ForwardVector" (`self.GetActorForwardVector`))))

(event `self.AIPerception.OnTargetPerceptionUpdated`
  (params (Actor :type "Actor Object Reference") (Stimulus :type "AIStimulus Structure")))

(event `MoveBackward`
  (`/Game/GoblinDreamLand/Core/BossGoblin/BP_BossGoblin.MoveToDirection` (`self.BossGoblin`) (* (`self.TackleTargetPoint`) -1.0)))

(event `TackleMoveStraight`
  ;[1 1 1] タックル関連処理
  ;;[1 1 1] タックル中の直進移動処理
  (`/Game/GoblinDreamLand/Core/BossGoblin/BP_BossGoblin.MoveToDirection` (`self.BossGoblin`) (`KismetMathLibrary.Normal` (`self.TackleTargetPoint`))))

(event `StopTackleProcess`
  ;[1 1 1] タックルを終わる時の処理
  (bind _asbp_boss_goblin (cast `/Game/GoblinDreamLand/Core/BossGoblin/BP_BossGoblin` (`self.K2_GetPawn`)))
  (`/Game/GoblinDreamLand/Core/BossGoblin/BP_BossGoblin.速さと加速度を初期値に設定` _asbp_boss_goblin))

(event `StartTackleProcess`
  ;[1 1 1] タックル関連処理
  ;;[1 1 1] タックルを始めるときの処理
  (`self.StopMovement`)
  (bind _asbp_boss_goblin (cast `/Game/GoblinDreamLand/Core/BossGoblin/BP_BossGoblin` (`self.K2_GetPawn`)))
  (set `self.BossGoblin` _asbp_boss_goblin)
  (set `self.TackleTargetPoint` (- (`self.K2_GetActorLocation` (`GameplayStatics.GetPlayerPawn` 0)) (`self.K2_GetActorLocation` (`self.BossGoblin`))))
  (`/Game/GoblinDreamLand/Core/BossGoblin/BP_BossGoblin.タックルの速さと加速度に変更` (`self.BossGoblin`)))

(fn `IsBrutal`
  (returns (IsBrutal :type Boolean))
  (bind _blackboardcomponent (`self.UseBlackboard` "/Game/GoblinDreamLand/Core/BossGoblin/BB_BossGoblin.BB_BossGoblin"))
  (return (`BlackboardComponent.GetValueAsBool` _blackboardcomponent "IsBrutal")))

(fn `UserConstructionScript`)

(fn `攻撃中か？`)