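; Boss goblin's thrown rock, launched on an arc aimed slightly short of the player and spinning in flight.
; BeginPlay pre-spawns a hidden BP_ExplosionRock, which Tick keeps matched to the rock's transform.
; A hit on anything but the player triggers breakup, immediately or after a delayed countdown depending on the first-hit flag.
; Breakup swaps in the Geometry Collection rock and destroys this actor; player overlap only prints.
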(event `Rotation`
  ;[1 1 1] 自身の回転
  (`self.K2_AddActorLocalRotation` (`KismetMathLibrary.RotatorFromAxisAndAngle` (`KismetMathLibrary.Cross_VectorVector` (`KismetMathLibrary.Normal` (`self.ThrowDirection`)) (0.0 0.0 1.0)) (* (`self.RotateSpeed`) (`GameplayStatics.GetWorldDeltaSeconds`)))))

(event `UpdateExplosionRock`
  ;[1 1 1] 爆発する岩のTRS更新
  (`self.K2_SetActorTransform` (`self.ExplosionRock`) (`self.GetTransform`) false false))

(event `SetFirstHitBreakFlag`
  (params (Flag :type Boolean))
  ;[1 1 1] 最初のヒットで破壊するか
  (set `self.IsFristHitBreak` Flag))

(event `self.ReceiveBeginPlay`
  (bind _outlaunchvelocity (`GameplayStatics.SuggestProjectileVelocity_CustomArc` (`self.K2_GetActorLocation`) (`self.K2_GetActorLocation` (`GameplayStatics.GetPlayerPawn` 0)) 0.0 0.7))
  (bind _output_get (set `self.ThrowDirection` (* _outlaunchvelocity (0.8 0.8 1.0))))
  (`PrimitiveComponent.AddImpulse` (`self.Rock-Mesh`) _output_get "None" true)
  (bind _returnvalue (`|SpawnActorFromClass` "/Game/GoblinDreamLand/Core/BossGoblin/Stone/BP_ExplosionRock.BP_ExplosionRock_C" (`self.GetTransform`) "Undefined" "MultiplyWithRoot" self null)) ; 爆発するほうも最初から生成しとくと
  (bind _output_get_2 (set `self.ExplosionRock` _returnvalue))
  (`self.SetActorHiddenInGame` _output_get_2 true) ; 見えないようにする
)

(event `self.ReceiveTick`
  (params (DeltaSeconds :type "Float (single-precision)"))
  (`self.UpdateExplosionRock`)
  (if (`self.IsHit`)
    (if (`self.IsFristHitBreak`)
      (`self.Explosion`)
      (else
        (`KismetSystemLibrary.Delay` 1.0)
        ;[1 1 1] タイマー処理
        (bind _result (`/Engine/EditorBlueprintResources/StandardMacros.DecrementInt` (`self.Timer`))
          (:`  `
            (if (<= _result 0)
              (`self.Explosion`))))))
    (else
      (`self.Rotation`))))

(event `Explosion`
  (bind _explosionrock (`self.ExplosionRock`))
  ;[1 1 1] 爆発処理
  (`/Engine/EditorBlueprintResources/StandardMacros.DoOnce` false
    (:`Completed`
      (`self.SetActorHiddenInGame` _explosionrock false)
      (`PrimitiveComponent.SetSimulatePhysics` (`GeometryCollectionActor.GeometryCollectionComponent` _explosionrock) true)
      (`/Game/GoblinDreamLand/Core/BossGoblin/Stone/BP_ExplosionRock.Explosion` _explosionrock)
      (`self.K2_DestroyActor`))))

(event `self.ReceiveActorBeginOverlap`
  (params (OtherActor :type "Actor Object Reference"))
  (bind _returnvalue (`KismetSystemLibrary.GetObjectName` OtherActor))
  ;[1 1 1] プレイヤーに当たったかはオーバーラップで判断
  (if (`KismetStringLibrary.EqualEqual_StrStr` (`KismetSystemLibrary.GetObjectName` (`GameplayStatics.GetPlayerPawn` 0)) _returnvalue)
    (`KismetSystemLibrary.PrintString` _returnvalue)))

(event `self.ReceiveHit`
  (params (MyComp :type "PrimitiveComponent Object Reference") (Other :type "Actor Object Reference") (OtherComp :type "PrimitiveComponent Object Reference") (bSelfMoved :type Boolean) (HitLocation :type "Vector Structure") (HitNormal :type "Vector Structure") (NormalImpulse :type "Vector Structure") (Hit :type "HitResult Structure (by ref)"))
  ;[1 1 1] 破壊するかの判定はHitで判定
  (if (not (`KismetStringLibrary.EqualEqual_StrStr` (`KismetSystemLibrary.GetObjectName` (`GameplayStatics.GetPlayerPawn` 0)) (`KismetSystemLibrary.GetObjectName` Other)))
    (set `self.IsHit` true) ; 地面にぶつかればヒットフラグをセット
  ))

(fn `UserConstructionScript`)