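; Sword-wielding player character that triggers slash and charged attacks through Gameplay Ability System tags.
; Punch input activates the slash; copy-attack input starts charging if the cooldown has expired, then fires the charge attack once past a hold threshold.
; An animation curve drives montage play rate during the charge, and Tick counts the cooldown down to zero.
; The construction script makes armor meshes follow the main mesh's pose via leader-pose components.
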(event `self.ReceiveTick`
  (params (DeltaSeconds :type "Float (single-precision)"))
  (`parent.ReceiveTick` DeltaSeconds)
  (bind _restcooltime (`self.CalcCoolTime` (`self.ChargeAttackCoolTime`) DeltaSeconds))
  (set `self.ChargeAttackCoolTime` _restcooltime))

(event `EnhancedInput|/Game/GoblinDreamLand/Core/Interactables/IA_Punch`
  (params (ActionValue :type Boolean) (ElapsedSeconds :type "Float (double-precision)") (TriggeredSeconds :type "Float (double-precision)") (InputAction :type "InputAction Object Reference" :default "/Game/GoblinDreamLand/Core/Interactables/IA_Punch.IA_Punch"))
  ;[1 1 1] 通常剣攻撃
  (:`Started`
    (`AbilitySystemComponent.TryActivateAbilitiesByTag` (`self.AbilitySystem`) (`BlueprintGameplayTagLibrary.MakeLiteralGameplayTagContainer` (struct :`GameplayTags` (struct :`(TagName` "Ability.Attack.SwordSlash")))) true)))

(event `EnhancedInput|/Game/GoblinDreamLand/Core/Interactables/IA_CopyAttack`
  (params (ActionValue :type Boolean) (ElapsedSeconds :type "Float (double-precision)") (TriggeredSeconds :type "Float (double-precision)") (InputAction :type "InputAction Object Reference" :default "/Game/GoblinDreamLand/Core/Interactables/IA_CopyAttack.IA_CopyAttack"))
  (bind _returnvalue (`SkeletalMeshComponent.GetAnimInstance` (`self.Mesh`)))
  ;[1 1 1] 特殊剣攻撃
  (:`Triggered`
    (if (`self.IsCanChargeAttack`)
      (if (< 0.38 ElapsedSeconds)
        (`/Engine/EditorBlueprintResources/StandardMacros.DoOnce` false :!label _label
          (:`Completed`
            (`AbilitySystemComponent.TryActivateAbilitiesByTag` (`self.AbilitySystem`) (`BlueprintGameplayTagLibrary.MakeLiteralGameplayTagContainer` (struct :`GameplayTags` (struct :`(TagName` "Ability.Attack.ChargeAttack")))) true)))
        (else
          (`AnimInstance.Montage_SetPlayRate` _returnvalue null 0.7) ; アニメ速度をリセットする
        ))))
  (:`Started`
    (if (<= (`self.ChargeAttackCoolTime`) 0.0)
      (set `self.IsCanChargeAttack` true)
      (`AbilitySystemComponent.TryActivateAbilitiesByTag` (`self.AbilitySystem`) (`BlueprintGameplayTagLibrary.MakeLiteralGameplayTagContainer` (struct :`GameplayTags` (struct :`(TagName` "Ability.Action.Charge")))) true)
      (else
        (set `self.IsCanChargeAttack` false))))
  (:`Ongoing`
    (if (`self.IsCanChargeAttack`)
      (`AnimInstance.Montage_SetPlayRate` _returnvalue null (`AnimInstance.GetCurveValue` _returnvalue "Chargeing")) ; チャージ中のアニメ速度をカーブで制御
      (set `self.ElapsedSecond` ElapsedSeconds)))
  (:`Completed`
    (goto _label :!via `Reset`)))

(fn `CalcCoolTime`
  (params (CoolTime :type "Float (double-precision)") (DeltaTime :type "Float (double-precision)"))
  (returns (RestCoolTime :type "Float (double-precision)"))
  (bind _returnvalue (- CoolTime DeltaTime))
  (if (<= _returnvalue 0.0)
    (return 0.0)
    (else
      (return _returnvalue))))

(fn `UserConstructionScript`
  (`SkinnedMeshComponent.SetLeaderPoseComponent` (`self.Helmet`) (`self.Mesh`) false false)
  (`SkinnedMeshComponent.SetLeaderPoseComponent` (`self.BodyArmor`) (`self.Mesh`) false false)
  (`SkinnedMeshComponent.SetLeaderPoseComponent` (`self.Bracers`) (`self.Mesh`) false false)
  (`SkinnedMeshComponent.SetLeaderPoseComponent` (`self.Skirt`) (`self.Mesh`) false false)
  (`SkinnedMeshComponent.SetLeaderPoseComponent` (`self.LegArmor`) (`self.Mesh`) false false))