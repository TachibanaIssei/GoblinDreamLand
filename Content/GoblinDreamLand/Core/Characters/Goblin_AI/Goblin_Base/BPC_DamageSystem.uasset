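; Damage and health component for the goblin AI, tracking health, death, invincibility and blocking.
; TakeDamage routes each hit through CanBeDamaged to block, damage or ignore it, honoring the DamageInfo override flags.
; It fires blocked, death or damage-response events, the latter only when interruptible or forced, and returns whether damage landed.
; Heal and both health getters are unfinished: Heal never changes Health and the getters return zero.
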(fn `GetCurrentHealth`
  (returns (Health :type "Float (double-precision)"))
  (return 0.0))

(fn `GetMaxHealth`
  (returns (MaxHealth :type "Float (double-precision)"))
  (return 0.0))

(fn `Heal`
  (params (Amount :type "Float (double-precision)" :default 0.0))
  (returns (NewHealth :type "Float (double-precision)"))
  (if (not (`self.IsDead`))
    (return 0.0)))

(fn `TakeDamage`
  (params (DamageInfo :type "/Game/GoblinDreamLand/Core/Characters/Goblin_AI/Goblin_Base/Struct/S_DamageInfo Structure") (DamageCauser :type "Actor Object Reference"))
  (returns (WasDamaged :type Boolean))
  (bind (_amount _damagetype _damageresponse _shoulddamageinvincible _canbeblocked _canbeparried _shouldforceinterrupt) (break `/Game/GoblinDreamLand/Core/Characters/Goblin_AI/Goblin_Base/Struct/S_DamageInfo` DamageInfo))
  (`self.CanBeDamaged` _shoulddamageinvincible _canbeblocked
    (:`BlockDamage`
      (`self.OnBlocked` _canbeparried)
      (return false))
    (:`DoDamage`
      (bind _output_get (set `self.Health` (- (`self.Health`) _amount)))
      (if (<= _output_get 0.0)
        (set `self.IsDead` true)
        (`self.OnDeath`)
        (elif (or (`self.IsInterrputible`) _shouldforceinterrupt)
          (`self.OnDamageResponse` _damageresponse DamageCauser)))
      (return true))
    (:`NoDamage`
      (return false))))