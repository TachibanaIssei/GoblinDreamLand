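; BP_StoneColumn is a stone column that rises while stood on and descends when vacated.
; Actor begin and end overlap events toggle a flag, without checking which actor overlaps.
; Tick moves the column one unit up or down per frame, unscaled by delta time.
; The tracked position is clamped between the BeginPlay location and a top point 1000 units above it.
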(event `self.ReceiveBeginPlay`
  ;[1 1 1] 初期座標と更新していく座標の設定
  (bind _output_get (set `self.FirstPosition` (`self.K2_GetActorLocation`)))
  (bind _output_get_2 (set `self.NewPosition` _output_get))
  ;[1 1 1] 頂上の座標の設定
  (set `self.TopPosition` (`KismetMathLibrary.MakeVector` (.x _output_get_2) (.y _output_get_2) (+ (.z _output_get_2) 1000.0))))

(event `self.ReceiveTick`
  (params (DeltaSeconds :type "Float (single-precision)"))
  ;[1 1 1] 柱に乗っているなら上昇し、乗っていないなら下降する
  (if (`self.IsOnCylinder`)
    (`self.K2_SetActorLocation` (+ (`self.NewPosition`) (0.0 0.0 1.0)))
    (else
      (`self.K2_SetActorLocation` (+ (`self.NewPosition`) (0.0 0.0 -1.0)))))
  (set `self.NewPosition` (`self.K2_GetActorLocation`))
  ;[1 1 1] 初期座標より下には下降しない
  (if (<= (.z (`self.NewPosition`)) (.z (`self.FirstPosition`)))
    (set `self.NewPosition` (`self.FirstPosition`))
    (else
      ;[1 1 1] 頂上の座標にたどり着いたらそれ以上上昇しない
      (if (>= (.z (`self.NewPosition`)) (.z (`self.TopPosition`)))
        (set `self.NewPosition` (`self.TopPosition`))))))

(event `self.ReceiveActorBeginOverlap`
  (params (OtherActor :type "Actor Object Reference"))
  ;[1 1 1] 柱に乗っているかのフラグを設定
  (set `self.IsOnCylinder` true))

(event `self.ReceiveActorEndOverlap`
  (params (OtherActor :type "Actor Object Reference"))
  ;[1 1 1] 柱に乗っているかのフラグを設定
  (set `self.IsOnCylinder` false))

(fn `UserConstructionScript`)