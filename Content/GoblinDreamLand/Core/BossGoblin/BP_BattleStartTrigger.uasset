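; Trigger volume actor that starts the goblin boss battle with an intro Level Sequence when the player pawn first overlaps it.
; It clears the boss's anim class and plays the sequence with the player hidden, binding the boss at runtime and using its world transform as the sequence origin through instance data.
; When the sequence finishes, it restores ABP_BossGoblin and calls BattleStart on the boss.
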(event `self.CollisionComponent.OnComponentBeginOverlap`
  (params (OverlappedComponent :type "PrimitiveComponent Object Reference") (OtherActor :type "Actor Object Reference") (OtherComp :type "PrimitiveComponent Object Reference") (OtherBodyIndex :type Integer) (bFromSweep :type Boolean) (SweepResult :type "HitResult Structure (by ref)"))
  (if (== OtherActor (`GameplayStatics.GetPlayerPawn` 0))
    (`/Engine/EditorBlueprintResources/StandardMacros.DoOnce` false
      (:`Completed`
        (`SkeletalMeshComponent.SetAnimInstanceClass` (`Character.Mesh` (`self.BossActor`)) null)
        (bind (_outactor _returnvalue) (`LevelSequencePlayer.CreateLevelSequencePlayer` (`self.BattleStartSequence`) (make `MovieSceneSequencePlaybackSettings` false (struct) 1.0 0.0 false false false true))) ; レベルシーケンスプレーヤーを作成
        (set `LevelSequenceActor.bOverrideInstanceData` true _outactor)
        (bind _asdefault_level_sequence_instance_data (cast `DefaultLevelSequenceInstanceData` (`LevelSequenceActor.DefaultInstanceData` _outactor)))
        (`LevelSequenceActor.AddBinding` _outactor (`|GetSequenceBinding` null) (`self.BossActor`) false) ; シーケンスのキャラクターを自身に変更
        (set `DefaultLevelSequenceInstanceData.TransformOrigin` (`SceneComponent.K2_GetComponentToWorld` (`Actor.RootComponent` (`self.BossActor`))) _asdefault_level_sequence_instance_data)
        (`MovieSceneSequencePlayer.Play` _returnvalue)
        (add `MovieSceneSequencePlayer.OnFinished` _returnvalue (delegate `カスタムイベント`))))))

(event `カスタムイベント`
  (`SkeletalMeshComponent.SetAnimInstanceClass` (`Character.Mesh` (`self.BossActor`)) "/Game/GoblinDreamLand/Core/BossGoblin/ABP_BossGoblin.ABP_BossGoblin_C")
  (`/Game/GoblinDreamLand/Core/BossGoblin/BP_BossGoblin.BattleStart` (`self.BossActor`)))

(fn `UserConstructionScript`)