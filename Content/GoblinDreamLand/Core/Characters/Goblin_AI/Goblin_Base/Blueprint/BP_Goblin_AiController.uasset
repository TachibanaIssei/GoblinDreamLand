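; AI controller for goblins that switches their blackboard state based on perception of the player.
; On possess, it stores the player as target, runs the pawn's behavior tree and starts Passive.
; Perception updates move Passive or Investigating goblins to Attacking when the player is seen within range, otherwise back to Passive.
; Hearing is a stub, damage only sets Passive, and StopAnimation halts the brain logic.
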(event `self.ReceivePossess`
  (params (PossessedPawn :type "Pawn Object Reference"))
  ;[1 1 1] ビヘイビアツリーとブラックボード使うための処理
  (bind _blackboardcomponent (`self.UseBlackboard` "/Game/GoblinDreamLand/Core/Characters/Goblin_AI/Goblin_Base/BB_Goblin_AI_base.BB_Goblin_AI_base"))
  (`BlackboardComponent.SetValueAsObject` _blackboardcomponent "TargetPlayer" (`GameplayStatics.GetPlayerPawn` 0))
  (bind _asbp_goblin_base (cast `/Game/GoblinDreamLand/Core/Characters/Goblin_AI/Goblin_Base/Blueprint/BP_Goblin_Base` PossessedPawn))
  (bind _behaviortrees (`/Game/GoblinDreamLand/Core/Characters/Goblin_AI/Goblin_Base/Blueprint/BP_Goblin_Base.BehaviorTrees` _asbp_goblin_base)
    (:`then`
      (`self.RunBehaviorTree` _behaviortrees)
      (`self.Set State as Passive` null))
    (:`else`)))

(event `self.AIPerception.OnPerceptionUpdated`
  (params (UpdatedActors :type "Array of Actor Object Reference (by ref)"))
  (bind _returnvalue (`GameplayStatics.GetPlayerPawn` 0))
  ;[1 1 1] 視野角を利用した処理
  (for _ UpdatedActors
    (`|ExecutionSequence`
      (:`then_0`
        (`self.Can Sense Actor` null "NewEnumerator1")
        (if true
          (if (<= (`KismetMathLibrary.VSize` (- (`self.K2_GetActorLocation`) (`self.K2_GetActorLocation` (`GameplayStatics.GetPlayerCharacter` 0)))) 1000.0)
            (`self.Handle Sensed Sight` _returnvalue)
            (else
              (`self.Set State as Passive` _returnvalue :!label _label)))
          (else
            (goto _label))))
      (:`then_1`
        (`self.Can Sense Actor` null "NewEnumerator2")
        (if true
          _))
      (:`then_2`
        (`self.Can Sense Actor` null "NewEnumerator3")
        (if true
          (`self.Handle Sensed Damege` null))))))

(event `StopAnimation`
  ;[1 1 1] AIの動作を止める
  (`BrainComponent.StopLogic` (`self.BrainComponent`) "")
  (cast `/Game/GoblinDreamLand/Core/Characters/Goblin_AI/Goblin_Base/Blueprint/BP_Goblin_Base` (`self.K2_GetPawn`)))

(fn `Can Sense Actor`
  (params (Actor :type "Actor Object Reference") (Sense :type "/Game/GoblinDreamLand/Core/Characters/Goblin_AI/Goblin_Base/enums/E_AISense Enum" :default "NewEnumerator0"))
  (returns (Sensed :type Boolean) (Stimulus :type "AIStimulus Structure"))
  (bind _info (`AIPerceptionComponent.GetActorsPerception` (`self.AIPerception`) Actor))
  (for _array_element (`.LastSensedStimuli` (break `ActorPerceptionBlueprintInfo` _info))
    (bind _returnvalue (`AIPerceptionSystem.GetSenseClassForStimulus` _array_element))
    (if (== _returnvalue (select `/Game/GoblinDreamLand/Core/Characters/Goblin_AI/Goblin_Base/enums/E_AISense` Sense :`NewEnumerator1` "/Script/AIModule.AISense_Sight" :`NewEnumerator2` "/Script/AIModule.AISenseConfig_Hearing" :`NewEnumerator3` "/Script/AIModule.AISense_Damage" :!type "Object Class Reference"))
      (return (`.bSuccessfullySensed` (break `AIStimulus` _array_element)) _array_element))))

(fn `Get Current States`
  (returns (NewParam :type "/Game/GoblinDreamLand/Core/Characters/Goblin_AI/Goblin_Base/enums/E_AiState Enum"))
  (return (cast `/Game/GoblinDreamLand/Core/Characters/Goblin_AI/Goblin_Base/enums/E_AiState` (`BlackboardComponent.GetValueAsEnum` (`self.Blackboard`) (`self.State Key Name`)))))

(fn `Handle Sensed Damege`
  (params (Actor :type "Actor Object Reference"))
  (bind _newparam (`self.Get Current States`))
  (switch `/Game/GoblinDreamLand/Core/Characters/Goblin_AI/Goblin_Base/enums/E_AiState` _newparam
    (:`NewEnumerator0`
      _)
    (:`NewEnumerator5`
      _))
  (`self.Set State as Passive` Actor))

(fn `Handle Sensed Sight`
  (params (Actor :type "Actor Object Reference"))
  (bind _newparam (`self.Get Current States`))
  (switch `/Game/GoblinDreamLand/Core/Characters/Goblin_AI/Goblin_Base/enums/E_AiState` _newparam
    (:`NewEnumerator0`
      _)
    (:`NewEnumerator2`
      _))
  (if (== Actor (`GameplayStatics.GetPlayerCharacter` 0))
    (`self.Set State as Attacking` Actor)))

(fn `Set State as Attacking`
  (params (TargetPlayer :type "Actor Object Reference"))
  (`BlackboardComponent.SetValueAsObject` (`self.Blackboard`) (`self.TargetPlayer`) TargetPlayer)
  (`BlackboardComponent.SetValueAsEnum` (`self.Blackboard`) (`self.State Key Name`) (enumliteral `/Game/GoblinDreamLand/Core/Characters/Goblin_AI/Goblin_Base/enums/E_AiState` "NewEnumerator1")))

(fn `Set State as Dead`
  (params (TargetPlayer :type "Actor Object Reference"))
  (`BlackboardComponent.SetValueAsEnum` (`self.Blackboard`) (`self.State Key Name`) (enumliteral `/Game/GoblinDreamLand/Core/Characters/Goblin_AI/Goblin_Base/enums/E_AiState` "NewEnumerator4")))

(fn `Set State as Passive`
  (params (Actor :type "Actor Object Reference"))
  (`BlackboardComponent.SetValueAsEnum` (`self.Blackboard`) (`self.State Key Name`) (enumliteral `/Game/GoblinDreamLand/Core/Characters/Goblin_AI/Goblin_Base/enums/E_AiState` "NewEnumerator0")))

(fn `UserConstructionScript`)