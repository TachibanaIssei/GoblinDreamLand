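; Stage gate actor with four panels that animate once, the first time any actor overlaps it.
; BeginPlay places the panels at fixed relative offsets on either side along X.
; On overlap, a DoOnce plays the GateTL timeline, whose single RightGate vector track is sign-flipped per panel to mirror the motion.
; Each update adds that vector to the panel's base offset plus ObjectPosition, which BeginPlay does not apply.
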(event `self.ReceiveBeginPlay`
  ;[1 1 1] 初期座標の設定
  (`SceneComponent.K2_SetRelativeLocation` (`self.GateR2`) (+ (0.0 0.0 0.0) (-900.0 0.0 0.0)) false false)
  (`SceneComponent.K2_SetRelativeLocation` (`self.GateR1`) (+ (0.0 0.0 0.0) (-920.0 0.0 0.0)) false false)
  (`SceneComponent.K2_SetRelativeLocation` (`self.GateL1`) (+ (0.0 0.0 0.0) (900.0 0.0 0.0)) false false)
  (`SceneComponent.K2_SetRelativeLocation` (`self.GateL2`) (+ (0.0 0.0 0.0) (920.0 0.0 0.0)) false false))

(event `self.ReceiveActorBeginOverlap`
  (params (OtherActor :type "Actor Object Reference"))
  (`/Engine/EditorBlueprintResources/StandardMacros.DoOnce` false
    (:`Completed`
      (bind (_direction _rightgate) (`Timeline|GateTL`)
        (:`Update`
          (`SceneComponent.K2_SetRelativeLocation` (`self.GateR2`) (+ (+ (* _rightgate (-1.0 -1.0 1.0)) (-900.0 0.0 0.0)) (`self.ObjectPosition`)) false false)
          (`SceneComponent.K2_SetRelativeLocation` (`self.GateR1`) (+ (+ (* _rightgate (-1.0 1.0 1.0)) (-920.0 0.0 0.0)) (`self.ObjectPosition`)) false false)
          (`SceneComponent.K2_SetRelativeLocation` (`self.GateL1`) (+ (+ (* _rightgate (1.0 1.0 1.0)) (900.0 0.0 0.0)) (`self.ObjectPosition`)) false false)
          (`SceneComponent.K2_SetRelativeLocation` (`self.GateL2`) (+ (+ (* _rightgate (1.0 -1.0 1.0)) (920.0 0.0 0.0)) (`self.ObjectPosition`)) false false))))))

(fn `UserConstructionScript`)