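; Player character Blueprint for the normal player variant, handling melee weapon and tackle hit detection.
; Right and left weapon collision overlaps apply fixed damage to the other actor and spawn a hit effect at its root component.
; Tackle overlaps call HitTackle on BP_TestEnemy.
; Each collision has its own DoOnce gate reset after a short delay, though a failed tackle cast never reaches that reset.
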(event `self.WeaponRCollision.OnComponentBeginOverlap`
  (params (OverlappedComponent :type "PrimitiveComponent Object Reference") (OtherActor :type "Actor Object Reference") (OtherComp :type "PrimitiveComponent Object Reference") (OtherBodyIndex :type Integer) (bFromSweep :type Boolean) (SweepResult :type "HitResult Structure (by ref)"))
  ;[1 1 1] 武器コリジョンに当たるとダメージを与える
  (`/Engine/EditorBlueprintResources/StandardMacros.DoOnce` false :!label _label
    (:`Completed`
      (`GameplayStatics.ApplyDamage` OtherActor 10.0)
      (`self.SpawnHitEffect` (`Actor.RootComponent` OtherActor))
      (`KismetSystemLibrary.Delay` 0.5)
      (goto _label :!via `Reset`))))

(event `self.WeaponLCollision.OnComponentBeginOverlap`
  (params (OverlappedComponent :type "PrimitiveComponent Object Reference") (OtherActor :type "Actor Object Reference") (OtherComp :type "PrimitiveComponent Object Reference") (OtherBodyIndex :type Integer) (bFromSweep :type Boolean) (SweepResult :type "HitResult Structure (by ref)"))
  ;[1 1 1] 武器コリジョンに当たるとダメージを与える
  (`/Engine/EditorBlueprintResources/StandardMacros.DoOnce` false :!label _label_2
    (:`Completed`
      (`GameplayStatics.ApplyDamage` OtherActor 10.0)
      (`self.SpawnHitEffect` (`Actor.RootComponent` OtherActor))
      (`KismetSystemLibrary.Delay` 0.5)
      (goto _label_2 :!via `Reset`))))

(event `self.TackleCollision.OnComponentBeginOverlap`
  (params (OverlappedComponent :type "PrimitiveComponent Object Reference") (OtherActor :type "Actor Object Reference") (OtherComp :type "PrimitiveComponent Object Reference") (OtherBodyIndex :type Integer) (bFromSweep :type Boolean) (SweepResult :type "HitResult Structure (by ref)"))
  ;[1 1 1] タックルの当たり判定
  (`/Engine/EditorBlueprintResources/StandardMacros.DoOnce` false :!label _label_3
    (:`Completed`
      (bind _asbp_test_enemy (cast `/Game/GoblinDreamLand/Core/Characters/Player/BP_TestEnemy` OtherActor))
      (`/Game/GoblinDreamLand/Core/Characters/Player/BP_TestEnemy.HitTackle` _asbp_test_enemy)
      (`KismetSystemLibrary.Delay` 0.5)
      (goto _label_3 :!via `Reset`))))

(fn `UserConstructionScript`
  (`parent.UserConstructionScript`))