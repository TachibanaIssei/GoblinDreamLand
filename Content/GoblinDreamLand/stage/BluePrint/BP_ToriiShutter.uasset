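; BP_ToriiShutter is a one-shot torii shutter that swings two placed static mesh actors when something overlaps it.
; BeginPlay stores both meshes' starting rotations.
; The first overlap, gated by DoOnce, plays a timeline whose RotValue is subtracted from one mesh's yaw and added to the other's, turning them in opposite directions like double doors.
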(event `self.ReceiveBeginPlay`
  (set `self.FirstRot7096` (`SceneComponent.GetSocketRotation` (`self.StaticMeshActor_7096`) "None"))
  (set `self.FirstRot7098` (`SceneComponent.GetSocketRotation` (`self.StaticMeshActor_7098`) "None")))

(event `self.ReceiveActorBeginOverlap`
  (params (OtherActor :type "Actor Object Reference"))
  (`/Engine/EditorBlueprintResources/StandardMacros.DoOnce` false
    (:`Completed`
      (bind (_direction _rotvalue) (`Timeline|タイムライン`)
        (:`Update`
          (`SceneComponent.K2_SetRelativeRotation` (`self.StaticMeshActor_7096`) (`KismetMathLibrary.MakeRotator` (.roll (`self.FirstRot7096`)) (.pitch (`self.FirstRot7096`)) (- (.yaw (`self.FirstRot7096`)) _rotvalue)) false false)
          (`SceneComponent.K2_SetRelativeRotation` (`self.StaticMeshActor_7098`) (`KismetMathLibrary.MakeRotator` (.roll (`self.FirstRot7098`)) (.pitch (`self.FirstRot7098`)) (+ _rotvalue (.yaw (`self.FirstRot7098`)))) false false))))))

(fn `UserConstructionScript`)