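; BP_woodbox is a stage wooden box actor that falls under its own scripted gravity along the Z axis only.
; While no overlap flags it as touching the floor, Tick accumulates airtime.
; Every tick it makes a swept move down by airtime times GravityStrength, so the fall accelerates.
; Any actor overlap toggles the floor flag, which only pauses the timer; airtime never resets and the downward move continues.
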(event `self.ReceiveTick`
  (params (DeltaSeconds :type "Float (single-precision)"))
  ;[1 1 1] 床についてないなら時間計測
  (if (not (`self.TouchFloor`))
    (bind _output_get (set `self.DeltaTime` (+ DeltaSeconds (`self.DeltaTime`)))))
  ;[1 1 1] Ｚ軸のみの重力を設定する
  (`self.K2_SetActorLocation` (`KismetMathLibrary.MakeVector` (.x (`self.K2_GetActorLocation`)) (.y (`self.K2_GetActorLocation`)) (- (.z (`self.K2_GetActorLocation`)) (* _output_get (`self.GravityStrength`)))) true))

(event `self.ReceiveActorBeginOverlap`
  (params (OtherActor :type "Actor Object Reference"))
  ;[1 1 1] 床についているかどうかを設定
  (set `self.TouchFloor` true))

(event `self.ReceiveActorEndOverlap`
  (params (OtherActor :type "Actor Object Reference"))
  ;[1 1 1] 床についているかどうかを設定
  (set `self.TouchFloor` false))

(fn `UserConstructionScript`)