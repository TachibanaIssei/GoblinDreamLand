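; BP_StoneBall is a stone projectile that flies along its negative local X axis and destroys both itself and any actor it hits.
; BeginPlay fixes the mesh to a large uniform scale, and Tick plays the Shake timeline.
; Timeline updates jitter the mesh on Y and Z by ShakeAmount, advance the actor without sweep, and accumulate elapsed time to destroy it after about three seconds.
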(event `self.ReceiveBeginPlay`
  ;[1 1 1] 弾の大きさを固定
  (`SceneComponent.SetWorldScale3D` (`self.StaticMeshComponent`) (28.0 28.0 28.0)))

(event `self.ReceiveTick`
  (params (DeltaSeconds :type "Float (single-precision)"))
  ;[1 1 1] タイムラインを使用して弾を振動させる
  (bind (_direction `_新規track_0`) (`Timeline|Shake`)
    (:`Update`
      (bind _returnvalue (* `_新規track_0` (`self.ShakeAmount`)))
      (`SceneComponent.K2_AddRelativeLocation` (`self.StaticMeshComponent`) (`KismetMathLibrary.Conv_Vector4ToVector` (`KismetMathLibrary.MakeVector4` 0.0 _returnvalue _returnvalue)) false false)
      (`self.K2_AddActorLocalOffset` (-15.0 0.0 0.0)) ; 前に飛ばされる
      ;[1 1 1] 時間経過で削除
      (set `self.ElapsedTime` (+ DeltaSeconds (`self.ElapsedTime`)))
      (if (> (`self.ElapsedTime`) 3.0)
        (`self.K2_DestroyActor`)))))

(event `self.ReceiveHit`
  (params (MyComp :type "PrimitiveComponent Object Reference") (Other :type "Actor Object Reference") (OtherComp :type "PrimitiveComponent Object Reference") (bSelfMoved :type Boolean) (HitLocation :type "Vector Structure") (HitNormal :type "Vector Structure") (NormalImpulse :type "Vector Structure") (Hit :type "HitResult Structure (by ref)"))
  ;[1 1 1] ぶつかったら消える
  (`self.K2_DestroyActor` Other)
  (`self.K2_DestroyActor`))

(fn `UserConstructionScript`)